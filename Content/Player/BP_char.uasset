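; Player character Blueprint that handles movement, camera look and jumping through Enhanced Input.
; On BeginPlay it adds the IMC_map mapping context, caches Llama from the GM_modo game mode and records its own transform there as PuntoDeSpawn, the spawn point.
; Movement follows control rotation, with forward using yaw only and right using yaw and roll, while look input drives controller yaw and pitch.
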(event `self.ReceiveBeginPlay`
  (bind _asgm_modo (cast `/Game/Blueprints/GM_modo` (`GameplayStatics.GetGameMode`) :!pure true))
  ;[1 1 1] Añadir mapping context
  (bind _asplayer_controller (cast `PlayerController` (`self.GetController`)))
  (bind _returnvalue (pcsubsystem `EnhancedInputLocalPlayerSubsystem` _asplayer_controller))
  (`/Engine/EditorBlueprintResources/StandardMacros.IsValid` _returnvalue
    (:`Is Valid`
      (`EnhancedInputSubsystemInterface.AddMappingContext` _returnvalue "/Game/Player/InputAction/IMC_map.IMC_map" 0 (struct))
      (bind _output_get (set `self.gamemode` _asgm_modo))
      (set `self.llama` (`/Game/Blueprints/GM_modo.llama` _output_get))
      (set `/Game/Blueprints/GM_modo.puntoDeSpawn` (`self.GetTransform`) _asgm_modo))))

(event `EnhancedInput|/Game/Player/InputAction/IA_movimiento`
  (params (ActionValue :type "Vector2D Structure") (ElapsedSeconds :type "Float (double-precision)") (TriggeredSeconds :type "Float (double-precision)") (InputAction :type "InputAction Object Reference" :default "/Game/Player/InputAction/IA_movimiento.IA_movimiento"))
  (bind (_returnvalue_roll _returnvalue_pitch _returnvalue_yaw) (`KismetMathLibrary.BreakRotator` (`self.GetControlRotation`)))
  ;[1 1 1] Movimiento. Modifica según dirección en X/Y y sentido en Z.
  (:`Triggered`
    (`self.AddMovementInput` (`KismetMathLibrary.GetRightVector` (`KismetMathLibrary.MakeRotator` _returnvalue_roll 0.0 _returnvalue_yaw)) ActionValue_X)
    (`self.AddMovementInput` (`KismetMathLibrary.GetForwardVector` (`KismetMathLibrary.MakeRotator` 0.0 0.0 _returnvalue_yaw)) ActionValue_Y)))

(event `EnhancedInput|/Game/Player/InputAction/IA_camara`
  (params (ActionValue :type "Vector2D Structure") (ElapsedSeconds :type "Float (double-precision)") (TriggeredSeconds :type "Float (double-precision)") (InputAction :type "InputAction Object Reference" :default "/Game/Player/InputAction/IA_camara.IA_camara"))
  ;[1 1 1] Control de cámara.
  (:`Triggered`
    (`self.AddControllerYawInput` ActionValue_X)
    (`self.AddControllerPitchInput` ActionValue_Y)))

(event `EnhancedInput|/Game/Player/InputAction/IA_salto`
  (params (ActionValue :type Boolean) (ElapsedSeconds :type "Float (double-precision)") (TriggeredSeconds :type "Float (double-precision)") (InputAction :type "InputAction Object Reference" :default "/Game/Player/InputAction/IA_salto.IA_salto"))
  ;[1 1 1] Salto
  (:`Triggered`
    (`self.Jump`))
  (:`Completed`
    (`self.StopJumping`)))

(fn `UserConstructionScript`)