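; BP_antorcha is a torch pickup actor that refills the flame value held by the game mode when the player touches it.
; On overlap with BP_char while lit, it calls AumentarLlama on GM_modo, hides its fire component and marks itself unlit.
; After a ten-second delay the fire reappears and the torch can be used again.
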(event `self.ReceiveBeginPlay`
  ;[1 1 1] Inicializa el estado encendido.
  (set `self.encendida` true))

(event `self.ReceiveActorBeginOverlap`
  (params (OtherActor :type "Actor Object Reference"))
  (bind _fuegotemporalaaaaaaaa (`self.FuegoTemporalAAAAAAAA`))
  ;[1 1 1] Si el jugador toca la antorcha, se modifica el valor de la variable llama en el gamemode y se oculta el componente fuego de la antorcha hasta transcurridos 10 segundos.
  (if (`self.encendida`)
    (cast `/Game/Player/BP_char` OtherActor)
    (`/Game/Blueprints/GM_modo.AumentarLlama` (cast `/Game/Blueprints/GM_modo` (`GameplayStatics.GetGameMode`) :!pure true))
    (`SceneComponent.SetHiddenInGame` _fuegotemporalaaaaaaaa true false)
    (set `self.encendida` false)
    (`KismetSystemLibrary.Delay` 10.0)
    (`SceneComponent.SetHiddenInGame` _fuegotemporalaaaaaaaa false false)
    (set `self.encendida` true)))

(fn `UserConstructionScript`)