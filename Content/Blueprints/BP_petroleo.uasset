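; BP_petroleo is an oil spill actor that appears and spreads after a BP_barrilPetroleo oil barrel overlaps it.
; The overlap destroys the barrel, waits briefly, then reveals the Plane and plays a Timeline.
; Each Timeline update cumulatively shifts the Plane and stretches it unevenly in X and Y using the Desplazamiento track.
; Overlapping a BP_destino actor stops the Timeline, halting the spread.
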(event `self.ReceiveActorBeginOverlap`
  (params (OtherActor :type "Actor Object Reference"))
  (bind (_returnvalue_location _returnvalue_rotation _returnvalue_scale) (`KismetMathLibrary.BreakTransform` (`SceneComponent.GetRelativeTransform` (`self.Plane`))))
  ;[1 1 1] Cuando detecta la colisión con el barril de petroleo, lo destruye, espera medio segundo, y comienza a expandirse en los ejes x e y según los parámetros definidos.
  (bind _asbp_barril_petroleo (cast `/Game/Blueprints/BP_barrilPetroleo` OtherActor)
    (:`then`
      (`self.K2_DestroyActor` _asbp_barril_petroleo)
      (`KismetSystemLibrary.Delay` 0.5)
      (`SceneComponent.SetVisibility` (`self.Plane`) true false)
      (bind (_direction _desplazamiento) (`Timeline|Timeline` :!label _label)
        (:`Update`
          (`SceneComponent.K2_SetRelativeTransform` (`self.Plane`) (`KismetMathLibrary.MakeTransform` (+ _returnvalue_location (0.2 0.4 0.0)) (struct) (+ _returnvalue_scale (`KismetMathLibrary.MakeVector` (* _desplazamiento 0.3) _desplazamiento))) false false))))
    (:`CastFailed`
      (cast `/Game/Blueprints/BP_destino` OtherActor)
      (goto _label :!via `Stop`))))

(fn `UserConstructionScript`)