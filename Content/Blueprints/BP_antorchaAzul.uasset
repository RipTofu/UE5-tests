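; BP_antorchaAzul is a blue torch that the player lights to lower bridges once enough flame is collected.
; When BP_char overlaps it, it checks whether Llama on the GM_modo game mode has reached 70, otherwise printing an insufficient-flame message.
; On success it loops over all BP_puente actors and, for array indices 2 and 3, shows Fuego and calls BajarPuente.
; Bridge selection depends on GetAllActorsOfClass ordering.
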(event `self.ReceiveActorBeginOverlap`
  (params (OtherActor :type "Actor Object Reference"))
  ;[1 1 1] Evalúa si se cumple la condición (La variable Llama debe haber alcanzado 70) recibiéndola desde el Gamemode. Si se cumple, itera sobre el array de actores de la clase puente, se encuentran los puentes de index 2 y 3, y se llama su respectivo evento "BajarPuente".
  (cast `/Game/Player/BP_char` OtherActor)
  (if (>= (`/Game/Blueprints/GM_modo.llama` (cast `/Game/Blueprints/GM_modo` (`GameplayStatics.GetGameMode`) :!pure true)) 70)
    (bind _outactors (`GameplayStatics.GetAllActorsOfClass` "/Game/Blueprints/BP_puente.BP_puente_C"))
    (for (_array_element _array_index) _outactors
      (if (and (<= _array_index 3) (>= _array_index 2))
        (`SceneComponent.SetVisibility` (`self.fuego`) true false)
        (`/Game/Blueprints/BP_puente.BajarPuente` _array_element)))
    (else
      (`KismetSystemLibrary.PrintString` "El nivel de la llama es insuficiente."))))

(fn `UserConstructionScript`)