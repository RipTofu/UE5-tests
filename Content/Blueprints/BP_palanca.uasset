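; BP_palanca is a lever that the player triggers by overlap to lower the first segment's bridges.
; A timeline applies incremental local pitch rotation to the actor while it plays.
; On finish it destroys the trigger, increments PartesCompletadas on the cached GM_modo game mode, and calls BajarPuente on the first two BP_puente actors found.
; Bridge selection relies on GetAllActorsOfClass array order rather than explicit references.
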(event `self.ReceiveBeginPlay`
  ;[1 1 1] Guarda gamemode como variable de la palanca.
  (set `self.gameMode` (cast `/Game/Blueprints/GM_modo` (`GameplayStatics.GetGameMode`) :!pure true)))

(event `self.ReceiveActorBeginOverlap`
  (params (OtherActor :type "Actor Object Reference"))
  (bind _gamemode (`self.gameMode`))
  ;[0.5505 1 0.5764] Verifica si el actor es el jugador. Ejecuta la rotación de palanca en un tiempo de 2.5 segundos modificando el eje Y. Luego, destruye la caja de colisión e incrementa la variable "partesCompletadas" del gamemode. Encuentra todos los elementos de la clase BP_puente y ejecuta la función Bajar Puente en los dos primeros (correspondientes al primer segmento del nivel).
  (if (`.bSuccess` (cast `/Game/Player/BP_char` OtherActor :!pure true))
    (bind (_direction _rotacion) (`Timeline|rotacionPalanca`)
      (:`Update`
        (`self.K2_AddActorLocalRotation` (`KismetMathLibrary.MakeRotator` 0.0 _rotacion)))
      (:`Finished`
        (`ActorComponent.K2_DestroyComponent` (`self.Trigger`))
        (bind _result (`/Engine/EditorBlueprintResources/StandardMacros.IncrementInt` (`/Game/Blueprints/GM_modo.partesCompletadas` _gamemode))
          (:`  `
            (set `/Game/Blueprints/GM_modo.partesCompletadas` _result _gamemode)
            (bind _outactors (`GameplayStatics.GetAllActorsOfClass` "/Game/Blueprints/BP_puente.BP_puente_C"))
            (for (_array_element _array_index) _outactors
              (if (<= _array_index 1)
                (`/Game/Blueprints/BP_puente.BajarPuente` _array_element)))))))))

(fn `UserConstructionScript`)